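; HUD Blueprint that shows score, time and level, plus a game-over screen with a "Press Enter" prompt.
; BeginPlay caches the Guide game mode and the first player state, looping back to retry the player state lookup while the stored reference is invalid.
; DrawHUD draws colored canvas text each frame, reading score and level from the player state, and time and the GameOver flag from the game mode.
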(event EventBeginPlay
  (bind _asbp_guide_gamemode (Utilities|Casting|CastToBP_Guide_Gamemode (Game|GetGameMode)))
  (Variables|Default|SetMy_Guide_GameMode _asbp_guide_gamemode)
  (bind _asbp_player_state (Utilities|Casting|CastToBP_PlayerState (Game|GetPlayerState 0) :!label _label))
  (Variables|Default|SetMy_PlayerState _asbp_player_state)
  (Utilities|IsValid (Variables|Default|GetMy_PlayerState)
    (:Is%20Not%20Valid
      (goto _label))))

(event Collision|EventActorBeginOverlap
  (params (OtherActor :type Actor%20Object%20Reference)))

(event EventTick
  (params (DeltaSeconds :type Float%20%28single-precision%29)))

(event EventDrawHUD
  (params (SizeX :type Integer) (SizeY :type Integer))
  (HUD|DrawText (Utilities|String|BuildString(Integer) "Score: " "" (Variables|/Game/BP_Guide/BP_PlayerState.BP_PlayerState_C|GetPlayerScore (Variables|Default|GetMy_PlayerState))) "(R=0.890478,G=1.000000,B=0.000000,A=1.000000)" 1e+01 1e+01 0 3.0 false)
  (HUD|DrawText (Utilities|String|BuildString(Integer) "Time: " "" (Variables|/Game/BP_Guide/BP_Guide_Gamemode.BP_Guide_Gamemode_C|GetTime (Variables|Default|GetMy_Guide_GameMode))) "(R=1.000000,G=0.000000,B=0.056713,A=1.000000)" 3e+02 1e+01 0 3.0 false)
  (HUD|DrawText (Utilities|String|BuildString(Integer) "Level: " "" (Variables|/Game/BP_Guide/BP_PlayerState.BP_PlayerState_C|GetLevel (Variables|Default|GetMy_PlayerState))) "(R=0.001826,G=0.000000,B=1.000000,A=1.000000)" 5.5e+02 1e+01 0 3.0 false)
  (if (Variables|/Game/BP_Guide/BP_Guide_Gamemode.BP_Guide_Gamemode_C|GetGameOver (Variables|Default|GetMy_Guide_GameMode))
    (HUD|DrawText "GAME OVER" "(R=1.000000,G=0.000000,B=0.025919,A=1.000000)" 4e+02 2e+02 0 3.0 false)
    (HUD|DrawText "Press Enter" "(R=1.000000,G=0.000000,B=0.025919,A=1.000000)" 4e+02 4e+02 0 3.0 false)))

(fn ConstructionScript)